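; Player1_BombArrival is a timed spawner that drops bombs from random points inside its Box.
; Tick counts TimeRemaining down, spawns a BombProjectile, then randomly sets its mesh, fuse Timer and slow downward velocity.
; Each bomb type sets the delay to the next spawn, but RandomInteger(2) only yields duck or dynamite, never the Nuke case.
; An ObjectArray shuffle that reveals hidden objects remains in the graph but never runs.
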(event `self.ReceiveBeginPlay`)

(event `self.ReceiveTick`
  (params (DeltaSeconds :type "Float (single-precision)"))
  (bind _box (`self.Box`))
  ;[1 1 1] Timer for how long till the next bomb spawns
  (bind _output_get (set `self.Time Remaining` (- (`self.Time Remaining`) (`GameplayStatics.GetWorldDeltaSeconds`))))
  (if (<= _output_get 0.0)
    ;[1 1 1] Shuffles the array so it randomly drops different bombs. The bool is used to reference in the bomb object. Reset Timer
    (bind _returnvalue (`|SpawnActorFromClass` "/Game/JoshFo/BombProjectile.BombProjectile_C" (`KismetMathLibrary.Conv_VectorToTransform` (`KismetMathLibrary.RandomPointInBoundingBox` (`SceneComponent.K2_GetComponentLocation` _box) (`BoxComponent.BoxExtent` _box))) "Undefined" "OverrideRootScale" null null))
    (switch `int` (`KismetMathLibrary.RandomInteger` 2)
      (:`0`
        (`StaticMeshComponent.SetStaticMesh` (`/Game/JoshFo/BombProjectile.Sphere` _returnvalue) "/Game/Bombs/DuckBomb.DuckBomb")
        (set `/Game/JoshFo/BombProjectile.Timer` 13.0 _returnvalue)
        (set `MovementComponent.Velocity` (0.0 0.0 -10.0) (`/Game/JoshFo/BombProjectile.ProjectileMovement` _returnvalue))
        (set `self.Time Remaining` 6.0))
      (:`1`
        (`StaticMeshComponent.SetStaticMesh` (`/Game/JoshFo/BombProjectile.Sphere` _returnvalue) "/Game/Bombs/Dynamite.Dynamite")
        (set `/Game/JoshFo/BombProjectile.Timer` 7.0 _returnvalue)
        (set `MovementComponent.Velocity` (0.0 0.0 -10.0) (`/Game/JoshFo/BombProjectile.ProjectileMovement` _returnvalue))
        (set `self.Time Remaining` 4.0))
      (:`2`
        (`StaticMeshComponent.SetStaticMesh` (`/Game/JoshFo/BombProjectile.Sphere` _returnvalue) "/Game/Bombs/Nuke.Nuke")
        (set `/Game/JoshFo/BombProjectile.Timer` 5.0 _returnvalue)
        (set `MovementComponent.Velocity` (0.0 0.0 -10.0) (`/Game/JoshFo/BombProjectile.ProjectileMovement` _returnvalue))
        (set `self.Time Remaining` 8.0)))))

(fn `UserConstructionScript`)