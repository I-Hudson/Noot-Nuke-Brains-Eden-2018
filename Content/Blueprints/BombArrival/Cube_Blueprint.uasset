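; Cube bomb actor for BombArrival that sets off a particle effect after a countdown once it lands on the floor.
; The mesh is hidden on BeginPlay, and a hit on an actor tagged Floor starts the timer, which Tick counts down.
; At zero it activates the particle system, then hides the mesh and stops the timer after a short delay.
; An unconnected fragment would lower the actor once BombArrival has spawned.
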(event `self.ReceiveBeginPlay`
  (`SceneComponent.SetVisibility` (`self.StaticMeshComponent`) false false))

(event `self.ReceiveTick`
  (params (DeltaSeconds :type "Float (single-precision)"))
  ;[1 1 1] If Run TImer is true reduce the timer untill it reachs 0
  (if (`self.Run Timer`)
    (set `self.Timer` (- (`self.Timer`) (`GameplayStatics.GetWorldDeltaSeconds`)))
    (if (<= (`self.Timer`) 0.0)
      (`ActorComponent.SetActive` (`self.ParticleSystem`) true false)
      (`KismetSystemLibrary.Delay` 0.2)
      (`SceneComponent.SetVisibility` (`self.StaticMeshComponent`) false false)
      (set `self.Run Timer` false))))

(event `self.StaticMeshComponent.OnComponentHit`
  (params (HitComponent :type "PrimitiveComponent Object Reference") (OtherActor :type "Actor Object Reference") (OtherComp :type "PrimitiveComponent Object Reference") (NormalImpulse :type "Vector Structure") (Hit :type "HitResult Structure (by ref)"))
  ;[1 1 1] When bomb hits the floor start the timer
  (if (`self.ActorHasTag` OtherActor "Floor")
    (set `self.Run Timer` true)))

(fn `UserConstructionScript`)