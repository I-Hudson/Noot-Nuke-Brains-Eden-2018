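; Bomb is an actor that the player throws as a physics sphere using keyboard input.
; Space launches it with a forward and upward impulse, while Left Shift stops physics and raises it for another throw.
; Hitting a "Floor"-tagged actor zeroes its velocity, and Tick pins it at the landing spot.
; An oscillating power-charge branch is never run, and the Map range-remap helper only feeds a Backspace debug print.
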(event `self.ReceiveBeginPlay`
  (`self.EnableInput` (`GameplayStatics.GetPlayerController` 0))
  (set `self.Land Location` (`SceneComponent.K2_GetComponentLocation` (`self.Sphere`)))
  (`SceneComponent.K2_SetWorldRotation` (`self.Sphere`) (`KismetMathLibrary.Conv_VectorToRotator` (0.0 90.0 0.0)) false false))

(event `self.ReceiveTick`
  (params (DeltaSeconds :type "Float (single-precision)"))
  (if (`self.On Ground`)
    (`SceneComponent.K2_SetWorldLocation` (`self.Sphere`) (`self.Land Location`) false false)))

(event `self.Sphere.OnComponentHit`
  (params (HitComponent :type "PrimitiveComponent Object Reference") (OtherActor :type "Actor Object Reference") (OtherComp :type "PrimitiveComponent Object Reference") (NormalImpulse :type "Vector Structure") (Hit :type "HitResult Structure (by ref)"))
  (bind _sphere (`self.Sphere`))
  (if (`self.ActorHasTag` OtherActor "Floor")
    (if (not (`self.On Ground`))
      (set `self.On Ground` true)
      (set `self.Land Location` (`SceneComponent.K2_GetComponentLocation` (`self.Sphere`)))
      (bind _asprimitive_component (cast `PrimitiveComponent` _sphere))
      (`PrimitiveComponent.SetAllPhysicsLinearVelocity` _sphere (0.0 0.0 0.0) false)
      (`PrimitiveComponent.SetAllPhysicsLinearVelocity` _asprimitive_component (0.0 0.0 0.0) false))
    (else
      (set `self.On Ground` false))))

(event `Key|SpaceBar`
  (params (Key :type "Key Structure"))
  (:`Released`
    (if (not (`self.On Ground`))
      (`PrimitiveComponent.SetSimulatePhysics` (`self.Sphere`) true)
      (`PrimitiveComponent.AddImpulse` (`self.Sphere`) (+ (* (`SceneComponent.GetForwardVector` (`self.Sphere`)) (* (`self.Forward Force`) 8.0)) (`KismetMathLibrary.MakeVector` 0.0 0.0 (* (`self.Up Force`) 1.0))) "None" false))))

(event `Key|LeftShift`
  (params (Key :type "Key Structure"))
  (:`Released`
    (`PrimitiveComponent.SetSimulatePhysics` (`self.Sphere`) false)
    (`SceneComponent.K2_SetWorldLocation` (`self.Sphere`) (+ (`SceneComponent.K2_GetComponentLocation` (`self.Sphere`)) (0.0 0.0 80.0)) false false)
    (set `self.On Ground` false)))

(event `Key|BackSpace`
  (params (Key :type "Key Structure"))
  (:`Released`
    (bind _output (`self.Map` 0.5 0.0 1.0 0.0 7.0))
    (`KismetSystemLibrary.PrintString` (`KismetStringLibrary.Conv_DoubleToString` _output))))

(fn `Map`
  (params (Value :type "Float (double-precision)") (Start1 :type "Float (double-precision)") (Stop1 :type "Float (double-precision)") (Start2 :type "Float (double-precision)") (Stop2 :type "Float (double-precision)"))
  (returns (Output :type "Float (double-precision)"))
  (locals (`v-start1` :type "Float (double-precision)") (`stop1-start1` :type "Float (double-precision)") (`stop2-start2` :type "Float (double-precision)") (firstValue :type "Float (double-precision)") (secondValue :type "Float (double-precision)"))
  (set `local.v-start1` (- Value Start1))
  (set `local.stop1-start1` (- Stop1 Start1))
  (set `local.stop2-start2` (- Stop2 Start2))
  (set `local.firstValue` (/ (`local.v-start1`) (`local.stop1-start1`)))
  (return (+ (* (`local.firstValue`) (`local.stop2-start2`)) Start2)))

(fn `UserConstructionScript`)